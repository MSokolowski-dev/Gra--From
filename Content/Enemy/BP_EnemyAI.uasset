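; BP_EnemyAI is a zombie enemy that detects pawns and performs a melee attack.
; PawnSensing sets the "seePlayer" Blackboard key for any seen pawn, as the Player tag check is unused, and nothing here clears it.
; AttackPlayer plays the attack montage and immediately sphere-traces forward from AttackTracePoints, damaging any pawn hit.
; An Attacking flag blocks repeat attacks until the montage completes.
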(event OnSeePawn(PawnSensing)
  (params (Pawn :type Pawn%20Object%20Reference))
  (if true
    (AI|Components|Blackboard|SetValueasBool (AI|GetBlackboard (AI|GetAIController self)) (Utilities|Name|MakeLiteralName "seePlayer") true)))

(event Custom|AttackPlayer
  (bind _attacktracepoints (Variables|Default|GetAttackTracePoints))
  (bind _returnvalue (Transformation|GetWorldLocation _attacktracepoints))
  (if (not (Variables|Default|Getattacking))
    (Variables|Default|Setattacking true)
    (Animation|Montage|PlayMontage (Variables|Character|GetMesh) "/Game/Enemy/Zombie_atac.Zombie_atac"
      (:then
        (bind (_outhit _returnvalue_2) (Collision|SphereTraceForObjects _returnvalue (+ _returnvalue (* (Math|Vector|GetForwardVector (Transformation|GetWorldRotation _attacktracepoints)) 7e+01)) 25.0 (Utilities|Array|MakeArray "ObjectTypeQuery3") false 0 "None"))
        (if _returnvalue_2
          (Game|Damage|ApplyDamage (.HitActor (Collision|BreakHitResult _outhit)) 1e+01 0 0)))
      (:OnCompleted
        (Variables|Default|Setattacking false)))))

(fn ConstructionScript)